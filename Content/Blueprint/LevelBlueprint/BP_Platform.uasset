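; BP_Platform is a moving platform that shuttles back and forth along a spline, pausing at each end.
; A timeline, rate-scaled by move speed over spline length, drives the mesh's location and optional pitch and yaw.
; A FlipFlop alternates play and reverse after each delay.
; The construction script applies the configurable mesh and scale, and places colored start and end labels, hiding the end one on short splines.
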(event `self.ReceiveBeginPlay`
  ;[0.05098 0.05098 0.05098] Set Play rate with speed and spline length
  (`TimelineComponent.SetPlayRate` (`self.Timeline_SmoothMove`) (* (/ 1.0 (`SplineComponent.GetSplineLength` (`self.Spline`))) (`self.MoveSpeed`)))
  (`self.Move`))

(event `Move`
  ;[0.05098 0.05098 0.05098] Move platform along spline points
  (`/Engine/EditorBlueprintResources/StandardMacros.FlipFlop`
    (:`A`
      ;;[0.05098 0.05098 0.05098] Smooth lerp between start pos and final pos by using timeline
      (bind (_direction _alpha) (`Timeline|Timeline_SmoothMove` :!label _label)
        (:`Update`
          (`|ExecutionSequence`
            (:`then_0`
              (bind _returnvalue (* _alpha (`SplineComponent.GetSplineLength` (`self.Spline`))))
              ;;[0.05098 0.05098 0.05098] Update relative location
              (`SceneComponent.K2_SetRelativeLocation` (`self.StaticMesh`) (`SplineComponent.GetLocationAtDistanceAlongSpline` (`self.Spline`) _returnvalue "Local") false false))
            (:`then_1`
              (bind (_returnvalue_roll _returnvalue_pitch _returnvalue_yaw) (`KismetMathLibrary.BreakRotator` (`SplineComponent.GetRotationAtDistanceAlongSpline` (`self.Spline`) _returnvalue "Local")))
              ;;[0.05098 0.05098 0.05098] Update relative rotation
              (`SceneComponent.K2_SetRelativeRotation` (`self.StaticMesh`) (`KismetMathLibrary.MakeRotator` (* _returnvalue_roll 0.0) (* (`self.UseRollAndPitch`) _returnvalue_pitch) (* _returnvalue_yaw (`self.UseYaw`))) false false))))
        (:`Finished`
          ;;[0.05098 0.05098 0.05098] Finished
          (`KismetSystemLibrary.Delay` (`self.WaitTime`))
          (`self.Move`))))
    (:`B`
      (goto _label :!via `Reverse`))))

(fn `UserConstructionScript`
  (bind _textstart (`self.TextStart`))
  (bind _spline (`self.Spline`))
  (bind _textend (`self.TextEnd`))
  (`|ExecutionSequence`
    (:`then_0`
      ;[0.05098 0.05098 0.05098] Set text settings
      ;;[0.05098 0.05098 0.05098] Set Start Text location and render color
      (`SceneComponent.K2_SetRelativeLocation` _textstart (`self.TextStartOffset`) false false)
      (`TextRenderComponent.SetTextRenderColor` _textstart (`self.TextColor`))
      ;;[0.05098 0.05098 0.05098] Set Visibility of text
      (if (> (`SplineComponent.GetSplineLength` (`self.Spline`)) 300.0)
        (`SceneComponent.SetVisibility` _textend true false)
        ;;[0.05098 0.05098 0.05098] Set Text End location to last spline poit and set render color
        (`SceneComponent.K2_SetRelativeLocation` _textend (+ (`self.TextEndOffset`) (`SplineComponent.GetLocationAtSplinePoint` _spline (`KismetMathLibrary.FTrunc` (`SplineComponent.GetSplineLength` _spline)) "Local")) false true)
        (`TextRenderComponent.SetTextRenderColor` _textend (`self.TextColor`))
        (else
          (`SceneComponent.SetVisibility` (`self.TextEnd`) false false))))
    (:`then_1`
      ;[0.05098 0.05098 0.05098] Set mesh
      (`StaticMeshComponent.SetStaticMesh` (`self.StaticMesh`) (`self.Mesh`))
      (`SceneComponent.SetRelativeScale3D` (`self.StaticMesh`) (`self.MeshScale`)))))