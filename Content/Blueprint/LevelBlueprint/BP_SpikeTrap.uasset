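; BP_SpikeTrap is a floor trap that raises spikes when a non-invincible player character stands in its trigger box.
; Timelines lerp the spikes' relative Z up and back down at configurable speeds, with delays before retracting and re-arming.
; Tick polls two boxes: one starts the trap while armed, the other applies damage once per cycle during the raised window.
; Invincibility is checked only on activation, not when damage is applied.
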(event `self.ReceiveBeginPlay`
  ;[0.05098 0.05098 0.05098] Set play speed
  (`TimelineComponent.SetPlayRate` (`self.Timeline_Activate`) (`self.ActivationSpeed`))
  (`TimelineComponent.SetPlayRate` (`self.Timeline_Deactivate`) (`self.DeactivateSpeed`)))

(event `ActivateTrap`
  (bind _spikes (`self.Spikes`))
  (bind (_relativelocation_x _relativelocation_y) (`KismetMathLibrary.BreakVector` (`SceneComponent.RelativeLocation` _spikes)))
  ;[0.05098 0.05098 0.05098] Trap
  ;;[0.05098 0.05098 0.05098] Activate Trap
  (set `self.Activate` false)
  (bind (_direction _alpha) (`Timeline|Timeline_Activate` :!via `PlayFromStart`)
    (:`Update`
      (`SceneComponent.K2_SetRelativeLocation` _spikes (`KismetMathLibrary.MakeVector` _relativelocation_x _relativelocation_y (`KismetMathLibrary.Lerp` -50.0 0.0 _alpha)) false false))
    (:`Finished`
      ;;;[0.05098 0.05098 0.05098] Finished
      (set `self.CanHitPlayer` true)
      (`KismetSystemLibrary.Delay` (`self.WaitTimeAfterActivate`))
      (set `self.CanHitPlayer` false)
      (`self.DeactivateTrap`))))

(event `self.ReceiveTick`
  (params (DeltaSeconds :type "Float (single-precision)"))
  (bind _returnvalue (`GameplayStatics.GetPlayerCharacter` 0))
  (bind _returnvalue_2 (`GameplayStatics.GetPlayerCharacter` 0))
  (`|ExecutionSequence`
    (:`then_0`
      ;[0.05098 0.05098 0.05098] Check if is overlapping player
      (if (`self.Activate`)
        (if (`PrimitiveComponent.IsOverlappingActor` (`self.TriggerBox1`) _returnvalue_2)
          (bind _asbp_player_character (cast `/Game/Blueprint/PlayerCharacter/BP_PlayerCharacter` _returnvalue_2))
          (if (not (`/Game/Blueprint/PlayerCharacter/BP_PlayerCharacter.IsInvicible` _asbp_player_character))
            (`self.ActivateTrap`)))))
    (:`then_1`
      ;[0.05098 0.05098 0.05098] Hit Player
      (if (`self.CanHitPlayer`)
        (if (`PrimitiveComponent.IsOverlappingActor` (`self.TriggerBox2`) _returnvalue)
          (`GameplayStatics.ApplyDamage` _returnvalue 1.0)
          (set `self.CanHitPlayer` false))))))

(event `DeactivateTrap`
  (bind _spikes (`self.Spikes`))
  (bind (_relativelocation_x _relativelocation_y) (`KismetMathLibrary.BreakVector` (`SceneComponent.RelativeLocation` _spikes)))
  ;[0.05098 0.05098 0.05098] Trap
  ;;[0.05098 0.05098 0.05098] Deactivate Trap
  (bind (_direction _alpha) (`Timeline|Timeline_Deactivate` :!via `PlayFromStart`)
    (:`Update`
      (`SceneComponent.K2_SetRelativeLocation` _spikes (`KismetMathLibrary.MakeVector` _relativelocation_x _relativelocation_y (`KismetMathLibrary.Lerp` 0.0 -50.0 _alpha)) false false))
    (:`Finished`
      ;;;[0.05098 0.05098 0.05098] Finished
      (`KismetSystemLibrary.Delay` (`self.WaitTimeBeforeActivate`))
      (set `self.Activate` true))))

(fn `UserConstructionScript`)