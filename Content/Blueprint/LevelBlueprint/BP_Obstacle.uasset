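; BP_Obstacle is a level obstacle with a configurable static mesh that gets pushed away from whatever actor interacts with it.
; The construction script applies the chosen Mesh to the component.
; Interactwith adds a horizontal impulse away from that actor, scaling ImpulseStrength by a float curve sampled at the clamped planar distance.
; The impulse is applied as a velocity change, so mass is ignored.
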(event `/Game/Blueprint/Other/BPI_Interactable.InteractWith`
  (params (Actor :type "Actor Object Reference"))
  (bind (_returnvalue_x _returnvalue_y) (`KismetMathLibrary.BreakVector` (- (`self.K2_GetActorLocation`) (`self.K2_GetActorLocation` Actor))))
  (bind _returnvalue (`KismetMathLibrary.MakeVector` _returnvalue_x _returnvalue_y))
  (`PrimitiveComponent.AddImpulse` (`self.StaticMesh`) (* (* (`KismetMathLibrary.Normal` _returnvalue) (`self.ImpulseStrength`)) (`CurveFloat.GetFloatValue` (`self.ImpulseScaleFromDist`) (`KismetMathLibrary.FClamp` (`KismetMathLibrary.VSize` _returnvalue) 0.0 250.0))) "None" true))

(fn `UserConstructionScript`
  (`StaticMeshComponent.SetStaticMesh` (`self.StaticMesh`) (`self.Mesh`)))