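; BP_WaterKillzone is a water hazard volume that respawns and damages the player who falls into it.
; Trigger overlap by the player character disables the trigger, blocks movement and spawns a foam splash at the player's location.
; After a configurable delay it calls Respawn, then applies damage shortly afterwards and re-enables the trigger.
; A timeline scales the splash emitter and destroys it when finished.
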(event `self.ReceiveBeginPlay`
  (`TimelineComponent.SetPlayRate` (`self.Timeline_SplashVFXScale`) 0.9))

(event `self.TriggerBox.OnComponentBeginOverlap`
  (params (OverlappedComponent :type "PrimitiveComponent Object Reference") (OtherActor :type "Actor Object Reference") (OtherComp :type "PrimitiveComponent Object Reference") (OtherBodyIndex :type Integer) (bFromSweep :type Boolean) (SweepResult :type "HitResult Structure (by ref)"))
  ;[0.05098 0.05098 0.05098] Player hit water
  (if (`self.EnableTrigger`)
    (bind _asbp_player_character (cast `/Game/Blueprint/PlayerCharacter/BP_PlayerCharacter` OtherActor))
    (set `self.EnableTrigger` false)
    (set `/Game/Blueprint/PlayerCharacter/BP_PlayerCharacter.CanMove` false _asbp_player_character)
    (`self.PlaySplashVFX` (`self.K2_GetActorLocation` _asbp_player_character))
    (`KismetSystemLibrary.Delay` (`self.DelayBeforeKill`))
    (`/Game/Blueprint/PlayerCharacter/BP_PlayerCharacter.Respawn` _asbp_player_character)
    (`KismetSystemLibrary.Delay` 0.1)
    (`GameplayStatics.ApplyDamage` _asbp_player_character 1.0)
    (set `self.EnableTrigger` true)))

(event `PlaySplashVFX`
  (params (Location :type "Vector Structure"))
  ;[0.05098 0.05098 0.05098] Splash effect
  (bind _returnvalue (`GameplayStatics.SpawnEmitterAtLocation` "/Game/Assets/CartoonWaterShader/Particles/PS_Waterfall_BottomFoam.PS_Waterfall_BottomFoam" Location (struct) (0.5 0.5 0.5) false))
  (bind (_direction _alpha) (`Timeline|Timeline_SplashVFXScale` :!via `PlayFromStart`)
    (:`Update`
      (`SceneComponent.SetWorldScale3D` _returnvalue (* (0.4 0.4 0.4) _alpha)))
    (:`Finished`
      (`ActorComponent.K2_DestroyComponent` _returnvalue))))

(fn `UserConstructionScript`)