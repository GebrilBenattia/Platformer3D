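; BP_Key is a collectible key pickup that animates along Z and carries a KeyType.
; A slowed timeline offsets the actor vertically from its starting location and restarts itself on finish to loop the motion.
; When a BP_PlayerCharacter overlaps the trigger sphere, the key passes its type to that character's GetKey and destroys itself.
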(event `self.ReceiveBeginPlay`
  (set `self.BaseLocation` (`self.K2_GetActorLocation`))
  (`TimelineComponent.SetPlayRate` (`self.Timeline_ZMove`) 0.3)
  (`self.Move`))

(event `Move`
  ;[0.05098 0.05098 0.05098] Move Z animation
  (bind (_direction _alpha) (`Timeline|Timeline_ZMove` :!via `PlayFromStart`)
    (:`Update`
      (`self.K2_SetActorLocation` (+ (`self.BaseLocation`) (`KismetMathLibrary.MakeVector` 0.0 0.0 (* _alpha 50.0)))))
    (:`Finished`
      (`self.Move`))))

(event `self.TriggerSphere.OnComponentBeginOverlap`
  (params (OverlappedComponent :type "PrimitiveComponent Object Reference") (OtherActor :type "Actor Object Reference") (OtherComp :type "PrimitiveComponent Object Reference") (OtherBodyIndex :type Integer) (bFromSweep :type Boolean) (SweepResult :type "HitResult Structure (by ref)"))
  ;[0.05098 0.05098 0.05098] Player get key
  (bind _asbp_player_character (cast `/Game/Blueprint/PlayerCharacter/BP_PlayerCharacter` OtherActor))
  (`/Game/Blueprint/PlayerCharacter/BP_PlayerCharacter.GetKey` _asbp_player_character (`self.KeyType`))
  (`self.K2_DestroyActor`))

(fn `UserConstructionScript`)