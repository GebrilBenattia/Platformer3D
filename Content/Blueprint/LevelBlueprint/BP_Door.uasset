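; BP_Door is a door locked by blue and yellow padlocks that opens once both matching keys are used.
; When a BP_PlayerCharacter enters its trigger box, each held key is consumed and its padlock starts simulating physics.
; Used keys are remembered across overlaps; once both are set, a timeline yaws the whole actor from its initial rotation, at a play rate set by RotationSpeed.
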(event `self.ReceiveBeginPlay`
  (set `self.BaseRotation` (`self.K2_GetActorRotation`))
  (`TimelineComponent.SetPlayRate` (`self.Timeline_OpenDoor`) (`self.RotationSpeed`)))

(event `self.Box.OnComponentBeginOverlap`
  (params (OverlappedComponent :type "PrimitiveComponent Object Reference") (OtherActor :type "Actor Object Reference") (OtherComp :type "PrimitiveComponent Object Reference") (OtherBodyIndex :type Integer) (bFromSweep :type Boolean) (SweepResult :type "HitResult Structure (by ref)"))
  (bind (_baserotation_roll _baserotation_pitch _baserotation_yaw) (`KismetMathLibrary.BreakRotator` (`self.BaseRotation`)))
  (if (not (`self.IsOpen`))
    (bind _asbp_player_character (cast `/Game/Blueprint/PlayerCharacter/BP_PlayerCharacter` OtherActor))
    (`|ExecutionSequence`
      (:`then_0`
        ;[0.05098 0.05098 0.05098] Use Blue key
        (if (`/Game/Blueprint/PlayerCharacter/BP_PlayerCharacter.HasBlueKey` _asbp_player_character)
          (`PrimitiveComponent.SetSimulatePhysics` (`self.SM_PadLockBlue`) true)
          (`/Game/Blueprint/PlayerCharacter/BP_PlayerCharacter.UseKey` _asbp_player_character "Blue")
          (set `self.BlueKeyUsed` true)))
      (:`then_1`
        ;[0.05098 0.05098 0.05098] Use Yellow Key
        (if (`/Game/Blueprint/PlayerCharacter/BP_PlayerCharacter.HasYellowKey` _asbp_player_character)
          (`PrimitiveComponent.SetSimulatePhysics` (`self.SM_PadLockYellow`) true)
          (`/Game/Blueprint/PlayerCharacter/BP_PlayerCharacter.UseKey` _asbp_player_character "Yellow")
          (set `self.YellowKeyUsed` true)))
      (:`then_2`
        (if (and (`self.BlueKeyUsed`) (`self.YellowKeyUsed`))
          (set `self.IsOpen` true)
          (bind (_direction _alpha) (`Timeline|Timeline_OpenDoor`)
            (:`Update`
              (`self.K2_SetActorRotation` (`KismetMathLibrary.MakeRotator` _baserotation_roll _baserotation_pitch (+ _baserotation_yaw (* _alpha (`self.ZMaxRotation`))))))))))))

(fn `UserConstructionScript`)