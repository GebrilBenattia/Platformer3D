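; Bumper level actor that launches any character entering its trigger sphere along the launch direction arrow's forward vector.
; After a short delay it halves the character's velocity and launches it, overriding XY only for the player character, then waits out a cooldown.
; Each launch bumps a scale factor that Tick spring-interpolates, giving the mesh a squash-and-stretch pop.
; The construction script applies mesh, scale and trigger placement.
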(event `self.ReceiveBeginPlay`
  ;[0.05098 0.05098 0.05098] Set base scaling
  (set `self.BaseScaling` (`SceneComponent.K2_GetComponentScale` (`self.StaticMesh`))))

(event `self.ReceiveTick`
  (params (DeltaSeconds :type "Float (single-precision)"))
  ;[0.05098 0.05098 0.05098] Scale with spring interp from scale factor
  (bind _returnvalue (`KismetMathLibrary.FloatSpringInterp` (`self.CurrentScaleFactor`) 0.0 (make `FloatSpringState`) 0.1 0.1 1.0 1.0 0.1 false -1.0 1.0 true))
  (set `self.CurrentScaleFactor` _returnvalue)
  (`SceneComponent.SetWorldScale3D` (`self.StaticMesh`) (+ (* (1.0 1.0 0.5) (`self.CurrentScaleFactor`)) (`self.BaseScaling`))))

(event `self.TriggerSphere.OnComponentBeginOverlap`
  (params (OverlappedComponent :type "PrimitiveComponent Object Reference") (OtherActor :type "Actor Object Reference") (OtherComp :type "PrimitiveComponent Object Reference") (OtherBodyIndex :type Integer) (bFromSweep :type Boolean) (SweepResult :type "HitResult Structure (by ref)"))
  ;[0.05098 0.05098 0.05098] Launch character whene overlap
  ;;[0.05098 0.05098 0.05098] Check actor and if can launch + wait for duration
  (bind _ascharacter (cast `Character` OtherActor))
  (if (`self.CanLaunch`)
    (set `self.CanLaunch` false)
    (`KismetSystemLibrary.Delay` (`self.DelayBeforeLaunch`))
    (`|ExecutionSequence`
      (:`then_0`
        (bind _charactermovement (`Character.CharacterMovement` _ascharacter))
        ;;[0.05098 0.05098 0.05098] Rescale character velocity
        (set `MovementComponent.Velocity` (* (`MovementComponent.Velocity` _charactermovement) 0.5) _charactermovement)
        ;;[0.05098 0.05098 0.05098] Launch the character
        (`Character.LaunchCharacter` _ascharacter (* (`SceneComponent.GetForwardVector` (`self.LaunchDirection`)) (`self.LaunchVelocity`)) (== _ascharacter "/Game/Blueprint/PlayerCharacter/BP_PlayerCharacter.BP_PlayerCharacter") true))
      (:`then_1`
        ;;[0.05098 0.05098 0.05098] Set scale factor + delay for next launch
        (set `self.CurrentScaleFactor` (`self.AdditionalScaleFactor`))
        (`KismetSystemLibrary.Delay` (`self.CanLaunchDelay`))
        (set `self.CanLaunch` true)))))

(fn `UserConstructionScript`
  (bind _triggersphere (`self.TriggerSphere`))
  (`StaticMeshComponent.SetStaticMesh` (`self.StaticMesh`) (`self.Mesh`))
  (`SceneComponent.SetRelativeScale3D` (`self.StaticMesh`) (`self.MeshScale`))
  (`SceneComponent.K2_SetRelativeLocation` _triggersphere (`self.TriggerOffset`) false true)
  (`SphereComponent.SetSphereRadius` _triggersphere (`self.TriggerRadius`) true))