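; BP_Heart is a health pickup that heals BP_PlayerCharacter by 1 on sphere overlap, then destroys itself.
; On BeginPlay it launches its Box with an impulse in a random horizontal direction plus an upward boost.
; Timelines animate the mesh relative to its construction-time transform: a yaw spin and scale beat trigger each other in a loop.
; A separate FlipFlop-driven timeline bobs it up and down.
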(event `self.ReceiveBeginPlay`
  (`|ExecutionSequence`
    (:`then_0`
      ;[0.05098 0.05098 0.05098] Set Animations Speed
      (`TimelineComponent.SetPlayRate` (`self.Timeline_Rotate`) 0.6)
      (`TimelineComponent.SetPlayRate` (`self.Timeline_Beat`) 2.0)
      (`TimelineComponent.SetPlayRate` (`self.Timeline_Translation`) 0.2))
    (:`then_1`
      (`self.RandomLaunch`)
      (`self.RotateAnimation`)
      (`self.TranslateAnimation`))))

(event `RotateAnimation`
  ;[0.05098 0.05098 0.05098] Animations
  ;;[0.05098 0.05098 0.05098] Rotate Animation
  (bind (_direction _alpha) (`Timeline|Timeline_Rotate` :!via `PlayFromStart`)
    (:`Update`
      (`SceneComponent.K2_SetRelativeRotation` (`self.StaticMesh`) (`KismetMathLibrary.MakeRotator` 0.0 0.0 (* _alpha 360.0)) false false))
    (:`Finished`
      (`self.BeatAnimation`))))

(event `BeatAnimation`
  ;[0.05098 0.05098 0.05098] Animations
  ;;[0.05098 0.05098 0.05098] Beat Animation
  (bind (_direction _alpha) (`Timeline|Timeline_Beat` :!via `PlayFromStart`)
    (:`Update`
      (`SceneComponent.SetRelativeScale3D` (`self.StaticMesh`) (+ (* (0.2 0.2 0.2) _alpha) (`self.BaseScale`))))
    (:`Finished`
      (`self.RotateAnimation`))))

(event `TranslateAnimation`
  ;[0.05098 0.05098 0.05098] Animations
  ;;[0.05098 0.05098 0.05098] Translate Animation
  (`/Engine/EditorBlueprintResources/StandardMacros.FlipFlop`
    (:`A`
      (bind (_direction _alpha) (`Timeline|Timeline_Translation` :!via `PlayFromStart` :!label _label)
        (:`Update`
          (`SceneComponent.K2_SetRelativeLocation` (`self.StaticMesh`) (+ (`self.BaseLocation`) (`KismetMathLibrary.MakeVector` 0.0 0.0 (* _alpha 50.0))) false false))
        (:`Finished`
          (`self.TranslateAnimation`))))
    (:`B`
      (goto _label :!via `ReverseFromEnd`))))

(event `self.Sphere.OnComponentBeginOverlap`
  (params (OverlappedComponent :type "PrimitiveComponent Object Reference") (OtherActor :type "Actor Object Reference") (OtherComp :type "PrimitiveComponent Object Reference") (OtherBodyIndex :type Integer) (bFromSweep :type Boolean) (SweepResult :type "HitResult Structure (by ref)"))
  (bind _asbp_player_character (cast `/Game/Blueprint/PlayerCharacter/BP_PlayerCharacter` OtherActor))
  (`/Game/Blueprint/PlayerCharacter/BP_PlayerCharacter.Heal` _asbp_player_character 1)
  (`self.K2_DestroyActor`))

(fn `RandomLaunch`
  (bind (_returnvalue_x _returnvalue_y) (`KismetMathLibrary.BreakVector` (`KismetMathLibrary.RandomUnitVector`)))
  (`PrimitiveComponent.AddImpulse` (`self.Box`) (* (`self.LaunchStrenght`) (+ (`KismetMathLibrary.Normal` (`KismetMathLibrary.MakeVector` _returnvalue_x _returnvalue_y)) (0.0 0.0 2.0))) "None" false))

(fn `UserConstructionScript`
  (bind _staticmesh (`self.StaticMesh`))
  (set `self.BaseScale` (`SceneComponent.RelativeScale3D` _staticmesh))
  (set `self.BaseLocation` (`SceneComponent.RelativeLocation` _staticmesh)))