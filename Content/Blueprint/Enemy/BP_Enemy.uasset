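; Melee enemy AI character that patrols, chases and attacks the player, then searches the last known position when sight is lost.
; Boolean states drive AIMoveTo, animations and PawnSensing vision, with obstacle line traces confirming visibility.
; Losing sight spawns a last-seen snapshot to seek, with text cues above the enemy signaling suspicion and alert.
; Nav links trigger arced jumps; death squashes the mesh and may drop a heart.
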(event `self.ReceiveBeginPlay`
  (`TextRenderComponent.K2_SetText` (`self.TextRender`) (`self.Reset`))
  (`TextRenderComponent.SetWorldSize` (`self.TextRender`) 100.0)
  (set `self.TimeToLostPlayer` 1.0)
  (`self.Patrol`))

(event `self.ReceiveActorBeginOverlap`
  (params (OtherActor :type "Actor Object Reference")))

(event `self.ReceiveTick`
  (params (DeltaSeconds :type "Float (single-precision)"))
  (if (<= (`self.Life`) 0)
    (set `self.Dead` true)
    (if (`self.Dead`)
      (set `CharacterMovementComponent.MaxWalkSpeed` 0.0 (`self.CharacterMovement`))
      (set `self.Seeking` false)
      (set `self.Patroling` false)
      (set `self.Chasing` false)
      (`self.KillEnemy`)
      (else
        (`self.RotateTextRendered` :!label _label)
        (if (`self.Seeking`)
          (`self.SetPawnSensingProperties` 60.0 9500.0))
        (if (`self.Patroling`)
          (`self.SetPawnSensingProperties` 80.0 3000.0))
        (if (`self.Chasing`)
          (`self.SetPawnSensingProperties` 100.0 9500.0)
          (bind _seeplayer (`self.DoNotSeePlayer`))
          (if _seeplayer
            _
            (elif (not (`self.Seeking`))
              (`KismetSystemLibrary.RetriggerableDelay` (`self.TimeToLostPlayer`))
              (`self.SpawnPlayerSnapshot`))))))
    (else
      (goto _label))))

(event `self.PawnSensing.OnSeePawn`
  (params (Pawn :type "Pawn Object Reference"))
  (bind _continue (`self.CanDestroySnapshot`))
  (if _continue
    _
    (else
      _))
  (if (`self.Patroling`)
    (set `self.IsAnimated` false)
    (set `self.Patroling` false))
  (if (`self.Seeking`)
    (set `self.Seeking` false))
  (if (`self.Chasing`)
    (`self.FollowPlayer` :!label _label_2)
    (else
      (`self.WaitAtFirstContact`)
      (`KismetSystemLibrary.Delay` 0.3)
      (bind _seeplayer (`self.DoNotSeePlayer`))
      (if _seeplayer
        (set `self.Patroling` true)
        (set `self.Idling` false)
        (else
          (`self.ChaseBeginingIndication`)
          (`KismetSystemLibrary.Delay` 1.0)
          (`TextRenderComponent.K2_SetText` (`self.TextRender`) (`self.Reset`))
          (goto _label_2))))))

(event `FollowPlayer`
  (if (`NavMovementComponent.IsFalling` (`self.CharacterMovement`))
    _
    (elif (`self.Chasing`)
      (if (`NavMovementComponent.IsFalling` (`Character.CharacterMovement` (`GameplayStatics.GetPlayerCharacter` 0)))
        _
        (else
          _))
      (`|AIMoveTo` self (0.0 0.0 0.0) (`GameplayStatics.GetPlayerController` 0) 50.0
        (:`then`
          (if (`PrimitiveComponent.IsOverlappingActor` (`self.DetectionBox`) (`GameplayStatics.GetPlayerCharacter` 0))
            (set `CharacterMovementComponent.MaxWalkSpeed` 950.0 (`self.CharacterMovement`))
            (`self.Attack`)
            (`KismetSystemLibrary.Delay` 0.7)
            (if (`PrimitiveComponent.IsOverlappingActor` (`self.HitBox`) (`GameplayStatics.GetPlayerCharacter` 0))
              (`GameplayStatics.ApplyDamage` (`GameplayStatics.GetPlayerCharacter` 0) 1.0)
              (`KismetSystemLibrary.Delay` 0.25)
              (else
                (`KismetSystemLibrary.Delay` 0.25)))
            (set `self.Attacking` false)
            (if (not (`self.Seeking`))
              (set `self.Chasing` true)
              (`self.FollowPlayer`))))
        (:`OnFail`
          (`self.Run`)
          (set `CharacterMovementComponent.MaxWalkSpeed` 700.0 (`self.CharacterMovement`)))))))

(event `MoveToNode`
  (params (Increment :type Integer))
  (if (`self.Patroling`)
    (`|AIMoveTo` self (0.0 0.0 0.0) (`|GetArrayItem` (`self.PatrolPath`) (`self.CurrentID`)) 7.0
      (:`then`
        (`self.Walk`)
        (set `CharacterMovementComponent.MaxWalkSpeed` 150.0 (`self.CharacterMovement`)))
      (:`OnSuccess`
        (bind _id (`self.IncrementPatrolCounter` Increment))
        (bind _output_get (set `self.CurrentID` _id))
        (if (== _output_get (- (`KismetArrayLibrary.Array_Length` (`self.PatrolPath`)) 1))
          (`self.MoveToNode` -1)
          (else
            (`self.MoveToNode` 1)))))))

(event `MoveToRandomNode`
  (if (`self.Patroling`)
    (bind _randompoint (`self.GetRandomPatrolPoint`))
    (bind _output_get (set `self.RandomPatrolPoint` _randompoint))
    (`|AIMoveTo` self _output_get null
      (:`then`
        (`self.Walk`)
        (set `CharacterMovementComponent.MaxWalkSpeed` 150.0 (`self.CharacterMovement`)))
      (:`OnSuccess`
        (`self.MoveToRandomNode`))
      (:`OnFail`
        (`KismetSystemLibrary.Delay` 15.0)
        (bind _randompoint_2 (`self.GetRandomPatrolPoint`))
        (set `self.RandomPatrolPoint` _randompoint_2)))))

(event `SeekToLastLocation`
  (if (`self.Patroling`)
    _
    (elif (`self.Seeking`)
      (`|AIMoveTo` self (`self.LastPlayerPos`) null
        (:`then`
          (bind _seeplayer (`self.DoNotSeePlayer`))
          (if (not _seeplayer)
            (bind _continue (`self.CanDestroySnapshot`))
            (if _continue
              (set `self.Seeking` false))))
        (:`OnSuccess`
          (`self.FinishingSeekingPlayer`))
        (:`OnFail`
          (bind _seeplayer_2 (`self.DoNotSeePlayer`))
          (if (not _seeplayer_2)
            (bind _continue_2 (`self.CanDestroySnapshot`))
            (if _continue_2
              (set `self.Seeking` false))))))))

(event `FinishingSeekingPlayer`
  (`self.CanDestroySnapshot`)
  (bind _seeplayer (`self.DoNotSeePlayer`))
  (if _seeplayer
    (set `self.Chasing` false)
    (bind _continue (`self.WaitAfterLoosingPlayer`))
    (if _continue
      (`KismetSystemLibrary.Delay` 1.5)
      (bind _continue_2 (`self.GettingAngryAfterLoosingPlayer`))
      (if _continue_2
        (`KismetSystemLibrary.Delay` 1.2)
        (bind _continue_3 (`self.ScreamAfterLoosingPlayer`))
        (if _continue_3
          (`KismetSystemLibrary.Delay` 1.0)
          (`self.ComeBackToPatrol`))))))

(event `/Game/Blueprint/Enemy/BPI_NavLinkReached.NavLinkInRange`
  (params (Destination :type "Vector Structure"))
  (if (not (`NavMovementComponent.IsFalling` (`self.CharacterMovement`)))
    (bind _outlaunchvelocity (`GameplayStatics.SuggestProjectileVelocity_CustomArc` (`self.K2_GetActorLocation`) Destination))
    (`self.LaunchCharacter` _outlaunchvelocity true true)
    (if (`self.Patroling`)
      (set `CharacterMovementComponent.MaxWalkSpeed` 500.0 (`self.CharacterMovement`))
      (`KismetSystemLibrary.Delay` 0.5))))

(event `KillEnemy`
  (if (`KismetSystemLibrary.IsValid` self)
    (if (`self.Dead`)
      (`TimelineComponent.SetPlayRate` (`self.Timeline_ScaleZ`) 0.7)
      (bind (_direction _alpha) (`Timeline|Timeline_ScaleZ`)
        (:`Update`
          (`SceneComponent.SetWorldScale3D` (`self.Mesh`) (+ (`KismetMathLibrary.Vector_One`) (`KismetMathLibrary.MakeVector` 0.0 0.0 (* _alpha -0.7)))))
        (:`Finished`
          (`GameplayStatics.SpawnEmitterAtLocation` "/Game/Assets/DreamscapeSeries2/DreamscapeTower/Effects/P_TeleportSparks.P_TeleportSparks" (`self.K2_GetActorLocation`) (struct) (0.5 0.5 0.5))
          (`self.SpawnHeartAtDeath` (`self.K2_GetActorLocation`))
          (`self.K2_DestroyActor`))))))

(event `self.ReceiveAnyDamage`
  (params (Damage :type "Float (single-precision)") (DamageType :type "DamageType Object Reference") (InstigatedBy :type "Controller Object Reference") (DamageCauser :type "Actor Object Reference"))
  (set `self.Life` (`KismetMathLibrary.FTrunc` (- (`self.Life`) Damage)))
  (if (<= (`self.Life`) 0)
    (`self.KillEnemy`)))

(fn `Attack`
  (if (`self.Attacking`)
    _
    (elif (`KismetMathLibrary.RandomBool`)
      (`SkeletalMeshComponent.PlayAnimation` (`self.Mesh`) "/Game/Assets/UndeadPack/EnemyGoblin/Animations/Anim_Attack1.Anim_Attack1" false)
      (set `self.Attacking` true)
      (set `self.IsAnimated` false)
      (else
        (`SkeletalMeshComponent.PlayAnimation` (`self.Mesh`) "/Game/Assets/UndeadPack/EnemyGoblin/Animations/Anim_Attack2.Anim_Attack2" false)
        (set `self.Attacking` true)
        (set `self.IsAnimated` false)))))

(fn `CanDestroySnapshot`
  (returns (Continue :type Boolean))
  (if (`KismetSystemLibrary.IsValid` (`self.LastPlayerSnapshot`))
    (`self.K2_DestroyActor` (`self.LastPlayerSnapshot`))
    (return true)))

(fn `ChaseBeginingIndication`
  (`SkeletalMeshComponent.PlayAnimation` (`self.Mesh`) "/Game/Assets/UndeadPack/EnemyGoblin/Animations/Anim_Agr.Anim_Agr" true)
  (`TextRenderComponent.SetTextRenderColor` (`self.TextRender`) (`self.ExclamationColor`))
  (`TextRenderComponent.K2_SetText` (`self.TextRender`) (`self.Exclamation`))
  (set `self.IsAnimated` false)
  (set `self.Attacking` false)
  (set `self.Idling` false)
  (set `self.Chasing` true))

(fn `ComeBackToPatrol`
  (bind _continue (`self.StopSeeking`))
  (if _continue
    (`self.SwitchToPatrol`)
    (`self.Patrol`)))

(fn `DoNotSeePlayer`
  (returns (seePlayer :type Boolean))
  (bind (_outhit _returnvalue) (`KismetSystemLibrary.LineTraceSingleForObjects` (`self.K2_GetActorLocation` self) (`self.K2_GetActorLocation` (`GameplayStatics.GetPlayerCharacter` 0)) (`self.Obstacle`)))
  (if _returnvalue
    _
    (else
      _))
  (return _returnvalue))

(fn `GetRandomPatrolPoint`
  (returns (RandomPoint :type "Vector Structure"))
  (return (`NavigationSystemV1.K2_GetRandomReachablePointInRadius` (`self.K2_GetActorLocation`) 1000.0 null null)))

(fn `GettingAngryAfterLoosingPlayer`
  (returns (Continue :type Boolean))
  (`self.ResetTextRendered`)
  (bind _continue (`self.StopSeeking`))
  (if _continue
    (`SkeletalMeshComponent.PlayAnimation` (`self.Mesh`) "/Game/Assets/UndeadPack/EnemyGoblin/Animations/Anim_Attack1.Anim_Attack1" false)
    (bind _continue_2 (`self.StopSeeking`))
    (if _continue_2
      (return true))))

(fn `Idle`
  (if (`self.Idling`)
    _
    (elif (not (`self.Attacking`))
      (`SkeletalMeshComponent.PlayAnimation` (`self.Mesh`) "/Game/Assets/UndeadPack/EnemyGoblin/Animations/Anim_Idle.Anim_Idle" true)
      (set `self.Idling` true)
      (set `self.Attacking` false))))

(fn `IncrementPatrolCounter`
  (params (Increment :type Integer))
  (returns (ID :type Integer))
  (return (`KismetMathLibrary.Clamp` (+ Increment (`self.CurrentID`)) 0 (- (`KismetArrayLibrary.Array_Length` (`self.PatrolPath`)) 1))))

(fn `JumpIn`
  (if (`self.IsAnimated`)
    _
    (elif (not (`self.Attacking`))
      (`SkeletalMeshComponent.PlayAnimation` (`self.Mesh`) "/Game/Assets/UndeadPack/EnemyGoblin/Animations/Anim_Jump_In.Anim_Jump_In" true)
      (set `self.IsAnimated` true)
      (set `self.Attacking` false))))

(fn `JumpOut`
  (if (`NavMovementComponent.IsFalling` (`self.CharacterMovement`))
    (if (`self.IsAnimated`)
      _
      (elif (not (`self.Attacking`))
        (`SkeletalMeshComponent.PlayAnimation` (`self.Mesh`) "/Game/Assets/UndeadPack/EnemyGoblin/Animations/Anim_Jump_In.Anim_Jump_In" true)
        (set `self.IsAnimated` true)
        (set `self.Attacking` false)))))

(fn `Patrol`
  (if (`KismetArrayLibrary.Array_IsNotEmpty` (`self.PatrolPath`))
    (set `self.Patroling` true)
    (`self.MoveToNode` 1)
    (else
      (set `self.Patroling` true)
      (`self.MoveToRandomNode`))))

(fn `ResetTextRendered`
  (`TextRenderComponent.K2_SetText` (`self.TextRender`) (`self.Reset`)))

(fn `RotateTextRendered`
  (`SceneComponent.K2_SetWorldRotation` (`self.TextRender`) (`KismetMathLibrary.FindLookAtRotation` (`self.K2_GetActorLocation`) (`self.K2_GetActorLocation` (`GameplayStatics.GetPlayerCharacter` 0))) false false))

(fn `Run`
  (if (`self.IsAnimated`)
    _
    (elif (not (`self.Attacking`))
      (`SkeletalMeshComponent.PlayAnimation` (`self.Mesh`) "/Game/Assets/UndeadPack/EnemyGoblin/Animations/Anim_Run.Anim_Run" true)
      (set `self.IsAnimated` true)
      (set `self.Attacking` false))))

(fn `ScreamAfterLoosingPlayer`
  (returns (Continue :type Boolean))
  (bind _continue (`self.StopSeeking`))
  (if _continue
    (`SkeletalMeshComponent.PlayAnimation` (`self.Mesh`) "/Game/Assets/UndeadPack/EnemyGoblin/Animations/Anim_Agr.Anim_Agr" false)
    (bind _continue_2 (`self.StopSeeking`))
    (if _continue_2
      (return true))))

(fn `SetPawnSensingProperties`
  (params (PeripheralVisionAngle :type "Float (double-precision)") (SightRadius :type "Float (double-precision)"))
  (`PawnSensingComponent.SetPeripheralVisionAngle` (`self.PawnSensing`) PeripheralVisionAngle)
  (set `PawnSensingComponent.SightRadius` SightRadius (`self.PawnSensing`)))

(fn `SetTextRendered`
  (params (Text :type Text) (TextColor :type "Color Structure"))
  (`TextRenderComponent.SetTextRenderColor` (`self.TextRender`) TextColor)
  (`TextRenderComponent.K2_SetText` (`self.TextRender`) Text))

(fn `SpawnHeartAtDeath`
  (params (Location :type "Vector Structure"))
  (if (<= (`KismetMathLibrary.RandomInteger` 100) 75)
    (`|SpawnActorFromClass` "/Game/Blueprint/LevelBlueprint/BP_Heart.BP_Heart_C" (`KismetMathLibrary.Conv_VectorToTransform` Location) "Undefined" "MultiplyWithRoot" null null)))

(fn `SpawnPlayerSnapshot`
  (bind _lastplayersnapshot (`self.LastPlayerSnapshot`))
  (bind _seeplayer (`self.DoNotSeePlayer`))
  (if _seeplayer
    (if (`KismetSystemLibrary.IsValid` _lastplayersnapshot)
      (`self.K2_DestroyActor` _lastplayersnapshot))
    (bind _output_get (set `self.LastPlayerPos` (`self.K2_GetActorLocation` (`GameplayStatics.GetPlayerCharacter` 0))))
    (bind _returnvalue (`|SpawnActorFromClass` "/Game/Blueprint/PlayerCharacter/BP_LastSeenIndicator.BP_LastSeenIndicator_C" (`KismetMathLibrary.Conv_VectorToTransform` _output_get) "DontSpawnIfColliding" "MultiplyWithRoot" null null))
    (bind _output_get_2 (set `self.LastPlayerSnapshot` _returnvalue))
    (`self.K2_SetActorRotation` _output_get_2 (`CharacterMovementComponent.GetLastUpdateRotation` (`Character.CharacterMovement` (`GameplayStatics.GetPlayerCharacter` 0))) false)
    (bind _seeplayer_2 (`self.DoNotSeePlayer`))
    (if _seeplayer_2
      (set `self.Seeking` true)
      (`self.SeekToLastLocation`)
      (elif (`KismetSystemLibrary.IsValid` (`self.LastPlayerSnapshot`))
        (`self.K2_DestroyActor` (`self.LastPlayerSnapshot`))
        (set `self.Seeking` false)))))

(fn `StopSeeking`
  (returns (Continue :type Boolean))
  (if (`self.Chasing`)
    (set `self.IsAnimated` false)
    (set `self.Seeking` false)
    (else
      (return true))))

(fn `SwitchToPatrol`
  (set `self.Patroling` true)
  (set `self.IsAnimated` false)
  (set `self.Chasing` false)
  (if (`KismetSystemLibrary.IsValid` (`self.LastPlayerSnapshot`))
    (`self.K2_DestroyActor` (`self.LastPlayerSnapshot`))
    (set `self.Seeking` false)))

(fn `UserConstructionScript`)

(fn `WaitAfterLoosingPlayer`
  (returns (Continue :type Boolean))
  (set `CharacterMovementComponent.MaxWalkSpeed` 0.0 (`self.CharacterMovement`))
  (`SkeletalMeshComponent.PlayAnimation` (`self.Mesh`) "/Game/Assets/UndeadPack/EnemyGoblin/Animations/Anim_Idle.Anim_Idle" false)
  (`self.SetTextRendered` (`self.Interogation`) (`self.InterogationColor`))
  (bind _continue (`self.StopSeeking`))
  (if _continue
    (return true)))

(fn `WaitAtFirstContact`
  (bind _seeplayer (`self.DoNotSeePlayer`))
  (if _seeplayer
    _
    (elif (not (`self.Idling`))
      (set `self.IsAnimated` false)
      (`self.Idle`)
      (set `CharacterMovementComponent.MaxWalkSpeed` 0.0 (`self.CharacterMovement`))
      (`self.SetTextRendered` (`self.Interogation`) (`self.InterogationColor`)))))

(fn `Walk`
  (if (`self.IsAnimated`)
    _
    (elif (not (`self.Attacking`))
      (`SkeletalMeshComponent.PlayAnimation` (`self.Mesh`) "/Game/Assets/UndeadPack/EnemyGoblin/Animations/Anim_Walk.Anim_Walk" true)
      (set `self.IsAnimated` true)
      (set `self.Attacking` false))))