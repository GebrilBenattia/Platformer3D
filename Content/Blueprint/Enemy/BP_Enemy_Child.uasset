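; Enemy child Blueprint that retreats to a heal zone to regenerate when hurt.
; Tick checks for Life below its starting value and, every frame while it is, flags regeneration and calls ComeBackToBase.
; That event stops chasing and uses AI MoveTo toward HealZone.
; On arrival, Regen idles, then restores Life and patrol state after a delay, while the Patrol check runs without waiting for that delay.
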(event `self.ReceiveBeginPlay`
  (set `self.Life` 2)
  (`parent.ReceiveBeginPlay`))

(event `self.ReceiveTick`
  (params (DeltaSeconds :type "Float (single-precision)"))
  (`parent.ReceiveTick` DeltaSeconds)
  (if (< (`self.Life`) 2)
    (set `self.NeedToRegen` true)
    (`self.ComeBackToBase`)))

(event `ComeBackToBase`
  (set `self.Chasing` false)
  (`|AIMoveTo` self (0.0 0.0 0.0) (`self.HealZone`)
    (:`OnSuccess`
      (`self.Regen`)
      (if (`self.Patroling`)
        (`self.Patrol`)))))

(event `Regen`
  (if (`self.NeedToRegen`)
    (set `self.IsAnimated` false)
    (`self.Idle`)
    (`KismetSystemLibrary.Delay` 5.0)
    (set `self.Life` 2)
    (set `self.IsAnimated` false)
    (set `self.Patroling` true)
    (set `self.NeedToRegen` false)))

(fn `UserConstructionScript`
  (`parent.UserConstructionScript`))